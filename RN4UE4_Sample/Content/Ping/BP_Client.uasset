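; BP_Client is a player-controlled client, apparently a Character, that drives a connection to a server for messaging and movement.
; It connects two seconds after BeginPlay; E sends a test message, and Q disconnects and destroys the actor.
; Non-zero movement axis values go to server-facing move functions defined outside this graph, while Jump is called directly with no server-named wrapper.
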(event `self.ReceiveBeginPlay`
  (`KismetSystemLibrary.Delay` 2.0)
  (`self.ConnectToServer`))

(event `Key|E`
  (params (Key :type "Key Structure" :default "AnyKey"))
  (:`Pressed`
    (`self.SendTestMessage`)))

(event `Key|Q`
  (params (Key :type "Key Structure" :default "AnyKey"))
  (:`Pressed`
    (`self.DisconnectFromServer`)
    (`self.K2_DestroyActor`)))

(event `InputAxis|MoveForward`
  (params (AxisValue :type "Float (single-precision)"))
  (if (!= AxisValue 0.0)
    (`self.MoveForwardServer` AxisValue)))

(event `InputAxis|MoveRight`
  (params (AxisValue :type "Float (single-precision)"))
  (if (!= AxisValue 0.0)
    (`self.MoveRightServer` AxisValue)))

(event `InputAction|Jump`
  (params (Key :type "Key Structure" :default "AnyKey"))
  (:`Pressed`
    (`self.Jump`)))

(fn `UserConstructionScript`)