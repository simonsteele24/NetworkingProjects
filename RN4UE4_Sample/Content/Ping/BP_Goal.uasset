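; BP_Goal is a goal actor that ends the match when a BP_BaseActor overlaps it.
; Only if the first BP_Client found is player 1, it calls DeclareWinner on the first BP_Server with the overlapping actor's player number.
; That client then enters post-game and is flagged as winner if the overlapping actor belongs to player 1.
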(event `self.ReceiveActorBeginOverlap`
  (params (OtherActor :type "Actor Object Reference"))
  (bind _asbp_base_actor (cast `/Game/Ping/BP_BaseActor` OtherActor))
  (bind _outactors (`GameplayStatics.GetAllActorsOfClass` "/Game/Ping/BP_Client.BP_Client_C"))
  (bind _item (`KismetArrayLibrary.Array_Get` _outactors))
  (if (== (`Client.playerNumber` _item) 1)
    (bind _outactors_2 (`GameplayStatics.GetAllActorsOfClass` "/Game/Ping/BP_Server.BP_Server_C"))
    (bind _playernum (`ReplicationActor.playerNum` _asbp_base_actor))
    (`Server.DeclareWinner` (`KismetArrayLibrary.Array_Get` _outactors_2) _playernum)
    (set `Client.bInPostGame` true _item)
    (set `Client.bIsWinner` (== _playernum 1) _item)))

(fn `UserConstructionScript`)