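; Camera pawn that follows the BP_BaseActor belonging to the client's player number.
; Three seconds after BeginPlay it destroys the first DefaultPawn, takes possession from player controller 0 and resolves its target once.
; The target is the BP_BaseActor whose PlayerNum matches the first BP_Client's PlayerNumber.
; Each Tick it copies that actor's location without sweep or smoothing, leaving rotation untouched.
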(event EventBeginPlay
  (Utilities|FlowControl|Delay 3.0)
  (bind _outactors (Actor|GetAllActorsOfClass "/Script/Engine.DefaultPawn"))
  (Actor|DestroyActor (Utilities|Array|Get(acopy) _outactors))
  (Pawn|Possess (Game|GetPlayerController 0) self)
  (CallFunction|GetPlayertoFollow))

(event Collision|EventActorBeginOverlap
  (params (OtherActor :type Actor%20Object%20Reference)))

(event EventTick
  (params (DeltaSeconds :type Float%20%28single-precision%29))
  (Utilities|IsValid (Variables|Default|GetPlayerToFollow)
    (:Is%20Valid
      (Transformation|SetActorLocation (Transformation|GetActorLocation (Variables|Default|GetPlayerToFollow)) false false))))

(fn ConstructionScript)

(fn GetPlayertoFollow
  (bind _outactors (Actor|GetAllActorsOfClass "/Game/Ping/BP_Client.BP_Client_C"))
  (LocalVariables|SetNum (Variables|/Script/RN4UE4_Sample.Client|GetplayerNumber (Utilities|Array|Get(acopy) _outactors)))
  (bind _outactors_2 (Actor|GetAllActorsOfClass "/Game/Ping/BP_BaseActor.BP_BaseActor_C"))
  (for _array_element _outactors_2
    (if (== (Variables|/Script/RN4UE4_Sample.ReplicationActor|GetplayerNum _array_element) (LocalVariables|GetNum))
      (Variables|Default|SetPlayerToFollow _array_element)
      (return))))